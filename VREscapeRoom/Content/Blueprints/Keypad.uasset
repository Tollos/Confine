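; VR keypad puzzle where the player enters a four-digit code to win a prize.
; Keypadhit matches the pressed key, fills four digit slots shown on the Code text, or resets them on Clear.
; A correct code plays celebration sounds, locks input and spawns the Prize.
; Wrong codes show remaining attempts; the third reveals animated hand meshes with a sound sting, then calls GameOver on Vr_Pawn.
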(event `/Game/VRInterface.Keypadhit`
  (params (NewParam :type "ActorComponent Object Reference") (`riGHT?` :type Boolean))
  (bind _returnvalue (`self.K2_GetActorLocation`))
  (bind _clear (`self.clear`))
  (bind _returnvalue_2 (`KismetStringLibrary.Conv_StringToInt` (`KismetStringLibrary.Conv_ObjectToString` (`self.NewVar_0`))))
  (if (not (`self.Won_0`))
    (set `self.NewVar_0` NewParam)
    (for _array_element (`|MakeArray` (`self.6`) (`self.1`) (`self.2`) (`self.3`) (`self.8`) (`self.4`) (`self.5`) (`self.9`) (`self.7`) _clear)
      (if (== _array_element (`self.NewVar_0`))
        (`GameplayStatics.PlaySoundAtLocation` "/Game/Sounds/SFX/Beep_1.Beep_1" (`self.K2_GetActorLocation`))
        (bind _output_get (set `self.NewVar_1` _array_element))
        (`|ExecutionSequence`
          (:`then_1`
            (if (not (== _clear _output_get))
              (if (== (`self.firstnumber`) 0)
                (bind _output_get_2 (set `self.firstnumber` _returnvalue_2))
                (`TextRenderComponent.K2_SetText` (`self.code`) (`KismetTextLibrary.Conv_StringToText` (`KismetStringLibrary.Concat_StrStr` (`KismetStringLibrary.Conv_IntToString` _output_get_2) "X" "X" "X")))
                (elif (== (`self.second number`) 0)
                  (bind _output_get_3 (set `self.second number` _returnvalue_2))
                  (`TextRenderComponent.K2_SetText` (`self.code`) (`KismetTextLibrary.Conv_StringToText` (`KismetStringLibrary.Concat_StrStr` (`KismetStringLibrary.Conv_IntToString` _output_get_2) (`KismetStringLibrary.Conv_IntToString` _output_get_3) "X" "X")))
                  (elif (== (`self.thirdnumber`) 0)
                    (bind _output_get_4 (set `self.thirdnumber` _returnvalue_2))
                    (`TextRenderComponent.K2_SetText` (`self.code`) (`KismetTextLibrary.Conv_StringToText` (`KismetStringLibrary.Concat_StrStr` (`KismetStringLibrary.Conv_IntToString` _output_get_2) (`KismetStringLibrary.Conv_IntToString` _output_get_3) (`KismetStringLibrary.Conv_IntToString` _output_get_4) "X")))
                    (elif (== (`self.fourthnumber`) 0)
                      (bind _output_get_5 (set `self.fourthnumber` _returnvalue_2))
                      (`|ExecutionSequence`
                        (:`then_0`
                          (`TextRenderComponent.K2_SetText` (`self.code`) (`KismetTextLibrary.Conv_StringToText` (`KismetStringLibrary.Concat_StrStr` (`KismetStringLibrary.Conv_IntToString` _output_get_2) (`KismetStringLibrary.Conv_IntToString` _output_get_3) (`KismetStringLibrary.Conv_IntToString` _output_get_4) (`KismetStringLibrary.Conv_IntToString` _output_get_5)))))
                        (:`then_1`
                          (if (and (and (== (`self.firstnumber`) (`self.answerOne`)) (== (`self.second number`) (`self.answerTwo`))) (and (== (`self.thirdnumber`) (`self.answerThree`)) (== (`self.fourthnumber`) (`self.answerFour`))))
                            (`GameplayStatics.PlaySoundAtLocation` "/Game/Sounds/SFX/Affirmative_Cue.Affirmative_Cue" _returnvalue)
                            (`GameplayStatics.PlaySoundAtLocation` "/Game/Sounds/Party_Blower.Party_Blower" _returnvalue)
                            (set `self.Won_0` true)
                            (`|SpawnActorFromClass` "/Game/Prize/Prize.Prize_C" (`KismetMathLibrary.MakeTransform` (0.0 0.0 0.0) (struct) (1.0 1.0 1.0)) "Undefined" "OverrideRootScale")
                            (else
                              (set `self.firstnumber` 0)
                              (set `self.second number` 0)
                              (set `self.thirdnumber` 0)
                              (set `self.fourthnumber` 0)
                              (bind _result (`/Engine/EditorBlueprintResources/StandardMacros.IncrementInt` (`self.Attempts`))
                                (:`  `
                                  (if (>= _result 3)
                                    (`GameplayStatics.PlaySound2D` "/Game/Sounds/Orchestral_Hit.Orchestral_Hit")
                                    (`SkeletalMeshComponent.PlayAnimation` (`self.SkeletalMesh`) "/Game/DirtyHands/HandAnim01_Anim.HandAnim01_Anim" false)
                                    (`SkeletalMeshComponent.PlayAnimation` (`self.SkeletalMesh3`) "/Game/DirtyHands/HandAnim01_Anim.HandAnim01_Anim" false)
                                    (`SkeletalMeshComponent.PlayAnimation` (`self.SkeletalMesh6`) "/Game/DirtyHands/HandAnim01_Anim.HandAnim01_Anim" false)
                                    (`SkeletalMeshComponent.PlayAnimation` (`self.SkeletalMesh1`) "/Game/DirtyHands/HandAnim03_Anim.HandAnim03_Anim" false)
                                    (`SkeletalMeshComponent.PlayAnimation` (`self.SkeletalMesh4`) "/Game/DirtyHands/HandAnim03_Anim.HandAnim03_Anim" false)
                                    (`SkeletalMeshComponent.PlayAnimation` (`self.SkeletalMesh7`) "/Game/DirtyHands/HandAnim02_Anim.HandAnim02_Anim" false)
                                    (`SkeletalMeshComponent.PlayAnimation` (`self.SkeletalMesh8`) "/Game/DirtyHands/HandAnim02_Anim.HandAnim02_Anim" false)
                                    (`SkeletalMeshComponent.PlayAnimation` (`self.SkeletalMesh2`) "/Game/DirtyHands/HandAnim02_Anim.HandAnim02_Anim" false)
                                    (`SkeletalMeshComponent.PlayAnimation` (`self.SkeletalMesh5`) "/Game/DirtyHands/HandAnim02_Anim.HandAnim02_Anim" false)
                                    (`KismetSystemLibrary.Delay` 0.1)
                                    (`SceneComponent.SetHiddenInGame` (`self.SkeletalMesh6`) false false)
                                    (`SceneComponent.SetHiddenInGame` (`self.SkeletalMesh`) false false)
                                    (`SceneComponent.SetHiddenInGame` (`self.SkeletalMesh3`) false false)
                                    (`SceneComponent.SetHiddenInGame` (`self.SkeletalMesh7`) false false)
                                    (`SceneComponent.SetHiddenInGame` (`self.SkeletalMesh8`) false false)
                                    (`SceneComponent.SetHiddenInGame` (`self.SkeletalMesh5`) false false)
                                    (`SceneComponent.SetHiddenInGame` (`self.SkeletalMesh2`) false false)
                                    (`SceneComponent.SetHiddenInGame` (`self.SkeletalMesh4`) false false)
                                    (`SceneComponent.SetHiddenInGame` (`self.SkeletalMesh1`) false false)
                                    (`KismetSystemLibrary.Delay` 0.75)
                                    (bind _asvr_pawn (cast `/Game/GameEssentails/Vr_Pawn` (`GameplayStatics.GetPlayerPawn` 0)))
                                    (`/Game/GameEssentails/Vr_Pawn.GameOver` _asvr_pawn)
                                    (else
                                      (`GameplayStatics.PlaySoundAtLocation` "/Game/Sounds/SFX/Negative.Negative" _returnvalue)
                                      (`KismetSystemLibrary.Delay` 0.2)
                                      (`TextRenderComponent.K2_SetText` (`self.code`) (`KismetSystemLibrary.MakeLiteralText` (`KismetTextLibrary.Conv_StringToText` (`KismetStringLibrary.Concat_StrStr` (`KismetStringLibrary.Conv_IntToString` (- 3 _result)) (select `bool` (not (== _result 1)) :`false` " attempts remain" :`true` " attempt remains")))))
                                      (`KismetSystemLibrary.Delay` 3.0)
                                      (`TextRenderComponent.K2_SetText` (`self.code`) "XXXX" :!label _label)))))))))))))
              (else
                (set `self.firstnumber` 0)
                (set `self.second number` 0)
                (set `self.thirdnumber` 0)
                (set `self.fourthnumber` 0)
                (goto _label)))))))))

(fn `UserConstructionScript`)