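; One-shot door Blueprint that creaks open for the VR player when ActivateBP fires.
; BeginPlay caches the Vr_Pawn and door position.
; Activation passes a DoOnce before checking the camera's world Y against the door with an offset, so a failed check still consumes it.
; On success it plays the creak, drives root yaw from a scaled timeline, sets Open and calls CallDoor.
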(event `/Game/VRInterface.activateBP`
  (`/Engine/EditorBlueprintResources/StandardMacros.DoOnce` false
    (:`Completed`
      (if (not (> (+ (.y (`SceneComponent.K2_GetComponentLocation` (`/Game/GameEssentails/Vr_Pawn.Camera` (`self.VRPawn`)))) -20.0) (.y (stale `self.ReceiveBeginPlay` _output_get))))
        (`|ExecutionSequence`
          (:`then_0`
            (`GameplayStatics.SpawnSoundAtLocation` "/Game/Sounds/Door_Creak_Cue.Door_Creak_Cue" (`SceneComponent.K2_GetComponentLocation` (`self.DefaultSceneRoot`)) (struct) 1.5)
            (bind (_direction _newtrack_0) (`Timeline|Timeline_0` :!via `PlayFromStart`)
              (:`Update`
                (`SceneComponent.K2_SetWorldRotation` (`self.DefaultSceneRoot`) (`KismetMathLibrary.MakeRotator` 0.0 0.0 (.z (* _newtrack_0 -0.75))) false false))))
          (:`then_1`
            (set `self.Open` true)
            (`self.Door` false)))))))

(event `self.ReceiveBeginPlay`
  (bind _asvr_pawn (cast `/Game/GameEssentails/Vr_Pawn` (`GameplayStatics.GetPlayerPawn` 0)))
  (set `self.VRPawn` _asvr_pawn)
  (bind _output_get (set `self.WorldLoc` (`SceneComponent.K2_GetComponentLocation` (`self.DefaultSceneRoot`)))))

(fn `UserConstructionScript`)