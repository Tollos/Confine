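; Compass actor that keeps its cone pointer at a fixed world orientation.
; Every Tick it forces the Cone component to a constant world rotation, then resets the actor's own rotation to zero.
; Disconnected leftover nodes hold earlier attempts to store the cone's rotation or pitch it with a look-at toward the actor's location.
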(event `self.ReceiveBeginPlay`)

(event `self.ReceiveTick`
  (params (DeltaSeconds :type "Float (single-precision)"))
  (`SceneComponent.K2_SetWorldRotation` (`self.Cone`) (struct :`Pitch` -90.0 :`Yaw` -90.0) false false)
  (`self.K2_SetActorRotation` (struct)))

(fn `UserConstructionScript`)