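; Blood decal actor that gives its decal a random blood splatter look.
; The construction script runs a random, looping MultiGate that sets the Decal component to one of twelve splatter materials.
; The event graph holds only disabled default events, so there is no runtime logic.
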(fn `UserConstructionScript`
  (bind _decal (`self.Decal`))
  (bind _decal_2 (`self.Decal`))
  (bind _decal_3 (`self.Decal`))
  (bind _decal_4 (`self.Decal`))
  (`|MultiGate` true true
    (:`Out 0`
      (`DecalComponent.SetDecalMaterial` _decal_2 "/Game/Blood/Blood_platter_v01.Blood_platter_v01"))
    (:`Out 1`
      (`DecalComponent.SetDecalMaterial` _decal_2 "/Game/Blood/Blood_platter_v02.Blood_platter_v02"))
    (:`Out 2`
      (`DecalComponent.SetDecalMaterial` _decal_2 "/Game/Blood/Blood_platter_v03.Blood_platter_v03"))
    (:`Out 3`
      (`DecalComponent.SetDecalMaterial` _decal_3 "/Game/Blood/Blood_platter_v04.Blood_platter_v04"))
    (:`Out 4`
      (`DecalComponent.SetDecalMaterial` _decal_3 "/Game/Blood/Blood_platter_v05.Blood_platter_v05"))
    (:`Out 5`
      (`DecalComponent.SetDecalMaterial` _decal_3 "/Game/Blood/Blood_platter_v06.Blood_platter_v06"))
    (:`Out 6`
      (`DecalComponent.SetDecalMaterial` _decal_4 "/Game/Blood/Blood_platter_v07.Blood_platter_v07"))
    (:`Out 7`
      (`DecalComponent.SetDecalMaterial` _decal_4 "/Game/Blood/Blood_platter_v08.Blood_platter_v08"))
    (:`Out 8`
      (`DecalComponent.SetDecalMaterial` _decal_4 "/Game/Blood/Blood_platter_v19.Blood_platter_v19"))
    (:`Out 9`
      (`DecalComponent.SetDecalMaterial` _decal "/Game/Blood/Blood_platter_v5sc.Blood_platter_v5sc"))
    (:`Out 10`
      (`DecalComponent.SetDecalMaterial` _decal "/Game/Blood/blood_splatter_dark_512.blood_splatter_dark_512"))
    (:`Out 11`
      (`DecalComponent.SetDecalMaterial` _decal "/Game/Blood/blood_splatter_lines.blood_splatter_lines"))))